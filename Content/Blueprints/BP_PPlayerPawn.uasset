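; BP_PPlayerPawn is a player pawn that sets up input and a camera view for its controller and passes movement input on.
; On BeginPlay it adds the IMC_BaseControlls Enhanced Input mapping context, then after a short delay blends the BP_PPlayerController view to a CameraActor found in the level.
; IA_Move input is forwarded to MoveServer, whose body is not defined in this file.
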(event Input|EnhancedActionEvents|EnhancedInputActionIA_Move
  (params (ActionValue :type Float%20%28double-precision%29) (ElapsedSeconds :type Float%20%28double-precision%29) (TriggeredSeconds :type Float%20%28double-precision%29) (InputAction :type Input%20Action%20Object%20Reference :default "/Game/Inputs/IA_Move.IA_Move"))
  (Class|PPlayerPawn|MoveServer ActionValue))

(event EventBeginPlay
  (|CallParentFunction)
  (bind _asplayer_controller (Utilities|Casting|CastToPlayerController (Pawn|GetController)))
  (Input|AddMappingContext (PlayerController|LocalPlayerSubsystems|GetEnhancedInputLocalPlayerSubsystem _asplayer_controller) "/Game/Inputs/IMC_BaseControlls.IMC_BaseControlls" 0 "(bIgnoreAllPressedKeysUntilRelease=True,bForceImmediately=False,bNotifyUserSettings=False)")
  (Utilities|FlowControl|Delay 1.0)
  (bind _returnvalue (Actor|GetActorOfClass "/Script/Engine.CameraActor"))
  (bind _asbp_pplayer_controller (Utilities|Casting|CastToBP_PPlayerController (Pawn|GetController)))
  (Game|Player|SetViewTargetwithBlend _asbp_pplayer_controller _returnvalue 0.1 "VTBlend_Linear" 0.0 false))

(fn ConstructionScript)